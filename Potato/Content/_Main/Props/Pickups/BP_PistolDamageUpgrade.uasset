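; Pickup that permanently removes itself when a character interacts with it, granting that character a pistol damage upgrade.
; Its Interact event adds DamageToAdd to the character's stored PistolDamage, then destroys the actor.
; A switch on the current weapon's name copies the new value into that weapon's Damage when it matches one entry, presumably the pistol, so an equipped weapon updates immediately.
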(event `/Game/_Main/Props/Pickups/BP_PickupMaster.Interact`
  (params (CharacterPickingUp :type "/Game/MetaHumans/Ettore/BP_Ettore Object Reference"))
  (bind _currentweapon (`/Game/MetaHumans/Ettore/BP_Ettore.CurrentWeapon` CharacterPickingUp))
  (bind _output_get (set `/Game/MetaHumans/Ettore/BP_Ettore.PistolDamage` (+ (`/Game/MetaHumans/Ettore/BP_Ettore.PistolDamage` CharacterPickingUp) (`self.DamageToAdd`)) CharacterPickingUp))
  (`self.K2_DestroyActor`)
  (switch `/Game/_Main/Props/Weapons/Enum_WeaponName` (`/Game/_Main/Props/Weapons/BP_weaponMaster.weaponName` _currentweapon)
    (:`NewEnumerator1`
      (set `/Game/_Main/Props/Weapons/BP_weaponMaster.Damage` _output_get _currentweapon))))

(fn `UserConstructionScript`
  (`parent.UserConstructionScript`))