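; Upgrade pickup that exposes a name and an escalating price for Assault damage, Health or Pistol damage upgrades.
; An UpgradeType switch selects the name and cost variable, with GetPrice truncating the cost to a whole number and SetPrice compounding it by 20% per call.
; GetPickup returns the actor itself, while GetDamage returns zero and CalcPrice is only a debug stub.
; The event graph is inactive, and applying the upgrade is not handled here.
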(fn `CalcPrice`
  (params (Target :type "/Game/_Main/Props/Pickups/I_BuyableObject Interface"))
  (`KismetSystemLibrary.PrintString` "Hello")
  (`self.getName`))

(fn `getDamage`
  (returns (damage :type "Float (double-precision)"))
  (return 0.0))

(fn `getName`
  (returns (name :type Text))
  (switch `/Game/_Main/Props/Pickups/Enum_UpgradeType` (`self.UpgradeType`)
    (:`NewEnumerator0`
      (return "Assult Damage Upgrade"))
    (:`NewEnumerator1`
      (return "Health Upgrade"))
    (:`NewEnumerator2`
      (return "Pistol Damage Upgrade"))))

(fn `getPickup`
  (returns (spawner :type "/Game/_Main/Props/Pickups/BP_PickupMaster Object Reference"))
  (return self))

(fn `getPrice`
  (returns (price :type Integer))
  (switch `/Game/_Main/Props/Pickups/Enum_UpgradeType` (`self.UpgradeType`)
    (:`NewEnumerator0`
      (return (`KismetMathLibrary.FTrunc` (`self.AssaultCost`))))
    (:`NewEnumerator1`
      (return (`KismetMathLibrary.FTrunc` (`self.HealthCost`))))
    (:`NewEnumerator2`
      (return (`KismetMathLibrary.FTrunc` (`self.PistolCost`))))))

(fn `setPrice`
  (returns (placeHolder :type Boolean))
  (switch `/Game/_Main/Props/Pickups/Enum_UpgradeType` (`self.UpgradeType`)
    (:`NewEnumerator0`
      (set `self.AssaultCost` (* (`self.AssaultCost`) 1.2)))
    (:`NewEnumerator1`
      (set `self.HealthCost` (* (`self.HealthCost`) 1.2)))
    (:`NewEnumerator2`
      (set `self.PistolCost` (* (`self.PistolCost`) 1.2))))
  (return true))

(fn `UserConstructionScript`
  (`parent.UserConstructionScript`))