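; BP_WeaponPickup is a world pickup that gives the interacting character a weapon.
; On Interact it calls SpawnWeapon on that character with its WeaponToSpawn, then destroys itself.
; Getters switch on WeaponName to report name, hardcoded price and damage for pistol or assault rifle, and GetPickup returns the actor itself.
; Damage is read from the player's BP_Ettore character rather than stored on the pickup, and Interact performs no price check.
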(event `/Game/_Main/Interface/BPI_Interact.Interact`
  (params (CharacterPickingUp :type "/Game/MetaHumans/Ettore/BP_Ettore Object Reference"))
  (`/Game/MetaHumans/Ettore/BP_Ettore.Spawn weapon` CharacterPickingUp (`self.WeaponToSpawn`))
  (`self.K2_DestroyActor`))

(fn `getDamage`
  (returns (damage :type "Float (double-precision)"))
  (bind _asbp_ettore (cast `/Game/MetaHumans/Ettore/BP_Ettore` (`GameplayStatics.GetPlayerCharacter` 0)))
  (switch `/Game/_Main/Props/Weapons/Enum_WeaponName` (`self.Weapon Name`)
    (:`NewEnumerator0`
      (return 0.0))
    (:`NewEnumerator1`
      (return (`/Game/MetaHumans/Ettore/BP_Ettore.PistolDamage` _asbp_ettore)))
    (:`NewEnumerator2`
      (return (`/Game/MetaHumans/Ettore/BP_Ettore.AssultDamage` _asbp_ettore)))))

(fn `getName`
  (returns (name :type Text))
  (switch `/Game/_Main/Props/Weapons/Enum_WeaponName` (`self.Weapon Name`)
    (:`NewEnumerator0`
      (return "Weapon"))
    (:`NewEnumerator1`
      (return "Pistol"))
    (:`NewEnumerator2`
      (return "Assault Rifle"))))

(fn `getPickup`
  (returns (spawner :type "/Game/_Main/Props/Pickups/BP_PickupMaster Object Reference"))
  (return self))

(fn `getPrice`
  (returns (price :type Integer))
  (switch `/Game/_Main/Props/Weapons/Enum_WeaponName` (`self.Weapon Name`)
    (:`NewEnumerator0`
      (return 0))
    (:`NewEnumerator1`
      (return 100))
    (:`NewEnumerator2`
      (return 1000))))

(fn `UserConstructionScript`
  (`parent.UserConstructionScript`))