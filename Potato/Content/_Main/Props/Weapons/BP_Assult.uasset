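; BP_Assult is an assault rifle weapon Blueprint that handles magazine ammo and the firing animation.
; Fire spends one round and plays the rifle fire animation on WeaponModel while ammo remains, with no trace, projectile or damage logic here.
; Reload sets the magazine from the passed reserve count, capped at MagSize, and returns the remainder, disregarding rounds already loaded.
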(event `/Game/_Main/Interface/BPI_Fire.Fire`
  (bind _ammoinweapon (`self.AmmoInWeapon`))
  (if (> _ammoinweapon 0)
    (`/Engine/EditorBlueprintResources/StandardMacros.DecrementInt` _ammoinweapon
      (:`  `
        (`SkeletalMeshComponent.PlayAnimation` (`self.WeaponModel`) "/Game/MilitaryWeapDark/Weapons/Anims/Fire_Rifle_W.Fire_Rifle_W" false)))))

(fn `Reload`
  (params (AmmoCount :type Integer))
  (returns (NewAmmoCount :type Integer))
  (locals (outAmmo :type Integer))
  (if (>= AmmoCount (`self.MagSize`))
    (set `self.AmmoInWeapon` (`self.MagSize`))
    (set `local.outAmmo` (- (`local.AmmoCount`) (`self.MagSize`)))
    (else
      (set `self.AmmoInWeapon` (`local.AmmoCount`))
      (set `local.outAmmo` 0)))
  (return (`local.outAmmo`)))

(fn `UserConstructionScript`
  (`parent.UserConstructionScript`))