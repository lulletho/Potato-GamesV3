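; Shop actor that lets the player open a weapon shop menu while standing in its overlap area.
; On BeginPlay it creates the prompt and shop HUD widgets, then spawns each class in Weapons far above itself and passes the instance to the HUD.
; Overlap toggles the prompt and an in-range flag that gates E to open and Q to close the HUD with the mouse cursor.
; Leaving the area also closes the shop.
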(event `self.ReceiveBeginPlay`
  (`self.createWidgets`))

(event `self.ReceiveActorBeginOverlap`
  (params (OtherActor :type "Actor Object Reference"))
  (if (== OtherActor (`GameplayStatics.GetPlayerCharacter` 0))
    (`UserWidget.AddToViewport` (`self.interactPrompt`) 0)
    (set `self.inRange` true)))

(event `self.ReceiveActorEndOverlap`
  (params (OtherActor :type "Actor Object Reference"))
  (if (== (`GameplayStatics.GetPlayerCharacter` 0) OtherActor)
    (`Widget.RemoveFromParent` (`self.interactPrompt`))
    (set `self.inRange` false)
    (`Widget.RemoveFromParent` (`self.HUD`))
    (set `PlayerController.bShowMouseCursor` false (`PlayerState.GetPlayerController` (`|GetArrayItem` (`GameStateBase.PlayerArray` (`GameplayStatics.GetGameState`)))))))

(event `Key|E`
  (params (Key :type "Key Structure"))
  (:`Pressed`
    (if (`self.inRange`)
      (`UserWidget.AddToViewport` (`self.HUD`) 0)
      (set `PlayerController.bShowMouseCursor` true (`PlayerState.GetPlayerController` (`|GetArrayItem` (`GameStateBase.PlayerArray` (`GameplayStatics.GetGameState`))))))))

(event `Key|Q`
  (params (Key :type "Key Structure"))
  (:`Pressed`
    (if (`self.inRange`)
      (`Widget.RemoveFromParent` (`self.HUD`))
      (set `PlayerController.bShowMouseCursor` false (`PlayerState.GetPlayerController` (`|GetArrayItem` (`GameStateBase.PlayerArray` (`GameplayStatics.GetGameState`))))))))

(fn `createWidgets`
  (bind _returnvalue (`|CreateWidget` "/Game/shop/shopPrompt.shopPrompt_C"))
  (set `self.interactPrompt` _returnvalue)
  (bind _returnvalue_2 (`|CreateWidget` "/Game/shop/shopHUD.shopHUD_C"))
  (bind _output_get (set `self.HUD` _returnvalue_2))
  (for _array_element (`self.weapons`)
    (bind _returnvalue_3 (`|SpawnActorFromClass` _array_element (`KismetMathLibrary.Conv_VectorToTransform` (+ (`self.K2_GetActorLocation`) (0.0 0.0 1000000000.0))) "AlwaysSpawn" "MultiplyWithRoot" null null))
    (`/Game/shop/shopHUD.addWeapon` _output_get _returnvalue_3)))

(fn `UserConstructionScript`)