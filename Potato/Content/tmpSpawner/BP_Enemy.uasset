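; BP_Enemy is a simple enemy that wanders at random and is destroyed when it takes any damage.
; From BeginPlay it moves with AIMoveTo to a random reachable point around its location, then repeats after a short delay.
; Only a successful move schedules the next one, so a failed move ends the wandering.
; On damage it destroys itself, then calls the OnDestroyed dispatcher.
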(event `self.ReceiveBeginPlay`
  (`self.Move`))

(event `Move`
  (`|AIMoveTo` self (`NavigationSystemV1.K2_GetRandomReachablePointInRadius` (`self.K2_GetActorLocation`) 2000.0 null null) null
    (:`OnSuccess`
      (`KismetSystemLibrary.Delay` 3.0)
      (`self.Move`))))

(event `self.ReceiveAnyDamage`
  (params (Damage :type "Float (single-precision)") (DamageType :type "DamageType Object Reference") (InstigatedBy :type "Controller Object Reference") (DamageCauser :type "Actor Object Reference"))
  (`self.K2_DestroyActor`)
  (`self.On Destroyed`))

(fn `UserConstructionScript`)