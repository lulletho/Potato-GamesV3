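; Enemy spawner that holds a queue of enemy classes and spawns them at random navigable points within a radius around itself.
; A looping timer spawns the front of the queue, while queueing an enemy also spawns immediately if no third-person character overlaps its sphere.
; Spawned actors get a destroy binding, and a defeat event forwards to the first-person game mode.
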(event `self.ReceiveBeginPlay`
  (`KismetSystemLibrary.K2_SetTimerDelegate` (delegate `TryToSpawn`) 2.0 true))

(event `TryToSpawn`
  (`self.SpawnEnemy`))

(event `OnEnemyDefeated`
  (bind _asbp_first_person_game_mode (cast `/Game/FirstPerson/Blueprints/BP_FirstPersonGameMode` (`GameplayStatics.GetGameMode`)))
  (`/Game/FirstPerson/Blueprints/BP_FirstPersonGameMode.OnEnemyDefeated` _asbp_first_person_game_mode))

(fn `Add Enemy to Queue`
  (params (EnemyClass :type "/Game/EnemyTest/ThirdPerson/Blueprints/BP_ThirdPersonCharacter Class Reference (by ref)"))
  (`KismetArrayLibrary.Array_Add` (`self.EnemyQueue`) EnemyClass)
  (if (not (`KismetArrayLibrary.Array_IsValidIndex` (`PrimitiveComponent.GetOverlappingActors` (`self.Sphere`) "/Game/EnemyTest/ThirdPerson/Blueprints/BP_ThirdPersonCharacter.BP_ThirdPersonCharacter_C")))
    (`self.SpawnEnemy`)))

(fn `SpawnEnemy`
  (returns (Success :type Boolean))
  (bind _returnvalue_location (`KismetMathLibrary.BreakTransform` (`self.GetTransform`)))
  (if (`KismetArrayLibrary.Array_IsValidIndex` (`self.EnemyQueue`))
    (bind _randomlocation (`NavigationSystemV1.K2_GetRandomLocationInNavigableRadius` _returnvalue_location (`self.Radius`) null null))
    (`|SpawnActorFromClass` (`|GetArrayItem` (`self.EnemyQueue`)) (`KismetMathLibrary.MakeTransform` _randomlocation) "AdjustIfPossibleButAlwaysSpawn" "MultiplyWithRoot" null null)
    (add `/Game/EnemyTest/ThirdPerson/Blueprints/BP_ThirdPersonCharacter.OnDestroy` (`|CreateDelegate` :!event `OnEnemyDefeated`))
    (`KismetArrayLibrary.Array_Remove` (`self.EnemyQueue`))
    (return true)
    (else
      (return false))))

(fn `UserConstructionScript`)